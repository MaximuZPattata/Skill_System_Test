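; Skill system component, by its name, that tracks cooldowns for Dash, Force Push and Invisibility; the skill effects themselves are not here, only debug prints.
; EnableSkillAbility rejects a skill whose IsActive flag is set in the Skills map, otherwise sets it and starts that skill's timer.
; Each skill has its own timer and completion event, which clears the flag through EnableSkillReady by rewriting the map entry with the same duration.
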(event Custom|Enable%20Skill%20Ability
  (params (Skill_Name :type ESkillNames%20Enum :default "NewEnumerator0"))
  (bind _skills (Variables|Default|GetSkills))
  (bind _value (Utilities|Map|Find _skills Skill_Name))
  (bind (_is_active _cooldown_duration) (Utilities|Struct|BreakST_SkillDetails _value))
  (if _is_active
    (Development|PrintString "Countdown still running")
    (else
      (CallFunction|SetSkillActivationBoolean true _cooldown_duration Skill_Name)
      (switch Utilities|FlowControl|Switch|SwitchonESkillNames Skill_Name
        (:NewEnumerator0
          (CallFunction|DashSkillTimerEvent _cooldown_duration Skill_Name)
          (Development|PrintString "Use Dash Skill"))
        (:NewEnumerator1
          (CallFunction|ForceSkillTimerEvent _cooldown_duration Skill_Name)
          (Development|PrintString "Use Force Skill"))
        (:NewEnumerator2
          (CallFunction|InvisibilitySkillTimerEvent _cooldown_duration Skill_Name)
          (Development|PrintString (Utilities|String|ToString(Float) _cooldown_duration)))))))

(event Custom|Dash%20Skill%20Cooldown%20Complete
  (CallFunction|EnableSkillReady false (stale Custom|Dash%20Skill%20Timer%20Event Cooldown%20Duration) (stale Custom|Dash%20Skill%20Timer%20Event Skill%20Name)))

(event Custom|Force%20Skill%20Cooldown%20Complete
  (CallFunction|EnableSkillReady false (stale Custom|Force%20Skill%20Timer%20Event Cooldown%20Duration) (stale Custom|Force%20Skill%20Timer%20Event Skill%20Name)))

(event Custom|Invisibility%20Skill%20Cooldown%20Complete
  (CallFunction|EnableSkillReady false (stale Custom|Invisibility%20Skill%20Timer%20Event Cooldown%20Duration) (stale Custom|Invisibility%20Skill%20Timer%20Event Skill%20Name)))

(event Custom|Dash%20Skill%20Timer%20Event
  (params (Cooldown%20Duration :type Float%20%28double-precision%29) (Skill%20Name :type ESkillNames%20Enum :default "NewEnumerator0"))
  (Utilities|Time|SetTimerbyEvent (delegate Custom|Dash%20Skill%20Cooldown%20Complete) Cooldown%20Duration))

(event Custom|Force%20Skill%20Timer%20Event
  (params (Cooldown%20Duration :type Float%20%28double-precision%29) (Skill%20Name :type ESkillNames%20Enum :default "NewEnumerator0"))
  (Utilities|Time|SetTimerbyEvent (delegate Custom|Force%20Skill%20Cooldown%20Complete) Cooldown%20Duration))

(event Custom|Invisibility%20Skill%20Timer%20Event
  (params (Cooldown%20Duration :type Float%20%28double-precision%29) (Skill%20Name :type ESkillNames%20Enum :default "NewEnumerator0"))
  (Utilities|Time|SetTimerbyEvent (delegate Custom|Invisibility%20Skill%20Cooldown%20Complete) Cooldown%20Duration)
  (Development|PrintString (Utilities|String|ToString(Float) Cooldown%20Duration)))

(fn SetSkillActivationBoolean
  (params (ActivateSkill :type Boolean) (CooldownTimer :type Float%20%28double-precision%29) (SkillName :type ESkillNames%20Enum :default "NewEnumerator0"))
  (Utilities|Map|Add (Variables|Default|GetSkills) SkillName (Utilities|Struct|MakeST_SkillDetails ActivateSkill CooldownTimer)))

(fn EnableSkillReady
  (params (ActivateSkill :type Boolean) (CooldownTimer :type Float%20%28double-precision%29) (SkillName :type ESkillNames%20Enum :default "NewEnumerator0"))
  (CallFunction|SetSkillActivationBoolean ActivateSkill CooldownTimer SkillName)
  (Development|PrintString "Skill ready to use"))